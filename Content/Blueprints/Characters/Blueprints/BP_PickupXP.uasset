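; BP_PickupXP is a pickup actor that hands its stored AmountXP to the player on contact.
; A box overlap checks that the other actor is a living BP_Player, then grants the amount through GainCoinMessage.
; It then resets the pickup transform and amount held in the game data from the GameInstance and destroys itself.
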(event `self.Box.OnComponentBeginOverlap`
  (params (OverlappedComponent :type "PrimitiveComponent Object Reference") (OtherActor :type "Actor Object Reference") (OtherComp :type "PrimitiveComponent Object Reference") (OtherBodyIndex :type Integer) (bFromSweep :type Boolean) (SweepResult :type "HitResult Structure (by ref)"))
  (if (== (`GameplayStatics.GetObjectClass` OtherActor) "/Game/Blueprints/Characters/Player/Blueprints/BP_Player.BP_Player_C")
    (bind _dead (message `/Game/Blueprints/Characters/Blueprints/Interface/BPI_Damagable.IsDead` OtherActor))
    (if (not _dead)
      (message `/Game/Blueprints/Characters/Blueprints/Interface/BPI_Coins.GainCoin` OtherActor (`self.AmountXP`))
      (bind _savegamedata (message `/Game/Blueprints/Save/BPI_SaveGame.GetGameData` (`GameplayStatics.GetGameInstance`)))
      (set `/Game/Blueprints/Save/BP_SaveGame.PickupXPTransforme` (`KismetMathLibrary.MakeTransform` (0.0 0.0 0.0)) _savegamedata)
      (set `/Game/Blueprints/Save/BP_SaveGame.PickupXPAmount` 0 _savegamedata)
      (`self.K2_DestroyActor`))))

(fn `UserConstructionScript`
  (`parent.UserConstructionScript`))