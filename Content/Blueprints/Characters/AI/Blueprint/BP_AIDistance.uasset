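; BP_AIDistance is a ranged AI character that attacks by firing projectiles.
; AutoAttack extends the parent, plays an attack montage, spawns a BP_Projectile ahead of the actor on the Attack notify, and calls AttackEnd on completion or interruption.
; Projectile impact is bound to DamageEnemy, which compares teams through messages, sends blockable, parryable damage to other teams and reports an AI damage event.
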(event `self.ReceiveBeginPlay`
  (`parent.ReceiveBeginPlay`))

(event `/Game/Blueprints/Characters/Blueprints/Interface/BPI_AIBase.AutoAttack`
  (params (AttackTarget :type "Actor Object Reference"))
  (`parent.AutoAttack` AttackTarget)
  (bind _notifyname (`|PlayMontage` (`self.Mesh`) "/Game/Blueprints/Characters/AI/Animations/AM_AIBaseAttackA.AM_AIBaseAttackA")
    (:`OnCompleted`
      (`/Game/Blueprints/Characters/Blueprints/Interface/BPI_AIBase.AttackEnd` AttackTarget :!label _label))
    (:`OnInterrupted`
      (goto _label))
    (:`OnNotifyBegin`
      (switch `name` _notifyname
        (:`Attack`
          (bind _returnvalue (`|SpawnActorFromClass` "/Game/Blueprints/Characters/Player/Blueprints/BP_Projectile.BP_Projectile_C" (`KismetMathLibrary.MakeTransform` (+ (`self.K2_GetActorLocation`) (* (`self.GetActorForwardVector`) 100.0)) (`self.K2_GetActorRotation`)) "Undefined" "MultiplyWithRoot" null 1500.0 0.0 null))
          (add `/Game/Blueprints/Characters/Player/Blueprints/BP_Projectile.OnProjectileImpact` _returnvalue (delegate `DamageEnemy`)))))))

(event `DamageEnemy`
  (params (OtherActor :type "Actor Object Reference") (Hit :type "HitResult Structure"))
  (bind _teamnumber (message `/Game/Blueprints/Characters/Blueprints/Interface/BPI_Damagable.GetTeamNumber` OtherActor))
  (bind _teamnumber_2 (message `/Game/Blueprints/Characters/Blueprints/Interface/BPI_Damagable.GetTeamNumber` self))
  (if (!= _teamnumber_2 _teamnumber)
    (message `/Game/Blueprints/Characters/Blueprints/Interface/BPI_Damagable.TakeDamage` OtherActor (make `/Game/Blueprints/Characters/Blueprints/Structures/S_DamageInfo` 40.0 "NewEnumerator2" "NewEnumerator1" false true true) self OtherActor)
    (`AISense_Damage.ReportDamageEvent` OtherActor self 10.0 (`self.K2_GetActorLocation`))))

(fn `UserConstructionScript`
  (`parent.UserConstructionScript`))