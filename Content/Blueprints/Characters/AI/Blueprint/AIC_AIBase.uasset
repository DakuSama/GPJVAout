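; Base AI controller that runs BT_AIBase and drives its blackboard state, attack target and the pawn-supplied attack and defend radii.
; Sight or damage perception of an actor on another team switches Passive or Idle AI to Attacking.
; A looping timer, started on possess, compares cached seen actors against perception to detect forgotten ones, returning to Passive when the attack target is lost.
; Pawn data and team numbers come through message calls.
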(event `self.ReceivePossess`
  (params (PossessedPawn :type "Pawn Object Reference"))
  (`self.RunBehaviorTree` "/Game/Blueprints/Characters/AI/BehaviorTree/BT_AIBase.BT_AIBase")
  (`self.SetStateAsPassive`)
  (`KismetSystemLibrary.Delay` 0.5)
  (bind (_attackradius _defendradius) (message `/Game/Blueprints/Characters/Blueprints/Interface/BPI_AIBase.GetIdealRange` PossessedPawn))
  (`BlackboardComponent.SetValueAsFloat` (`self.Blackboard`) (`self.AttackRadiusKeyName`) _attackradius)
  (`BlackboardComponent.SetValueAsFloat` (`self.Blackboard`) (`self.DefendRadiusKeyName`) _defendradius)
  (bind _returnvalue (`KismetSystemLibrary.K2_SetTimerDelegate` (`|CreateDelegate` :!event `CheckIfForgottenSeenActor`) 0.5 true))
  (set `self.CheckforgottenActorsTimer` _returnvalue))

(event `self.AIPerception.OnPerceptionUpdated`
  (params (UpdatedActors :type "Array of Actor Object Reference (by ref)"))
  (for _array_element UpdatedActors
    (`|ExecutionSequence`
      (:`then_0`
        (bind _sensed (`self.CanSenseActor` _array_element "NewEnumerator1"))
        (if _sensed
          (`self.HandleSensedSight` _array_element)))
      (:`then_1`
        (bind _sensed_2 (`self.CanSenseActor` _array_element "NewEnumerator2"))
        (if _sensed_2
          (`self.HandleSenseDamage` _array_element))))))

(event `self.ReceiveUnPossess`
  (params (UnpossessedPawn :type "Pawn Object Reference"))
  (`KismetSystemLibrary.K2_ClearAndInvalidateTimerHandle` (`self.CheckforgottenActorsTimer`)))

(event `CheckIfForgottenSeenActor`
  (if (!= (`KismetArrayLibrary.Array_Length` (`self.KnownSeenActors`)) (`KismetArrayLibrary.Array_Length` (`AIPerceptionComponent.GetKnownPerceivedActors` (`self.AIPerception`) "/Script/AIModule.AISense_Sight")))
    (for _array_element (`self.KnownSeenActors`)
      (if (== (`KismetArrayLibrary.Array_Find` (`AIPerceptionComponent.GetKnownPerceivedActors` (`self.AIPerception`) null) _array_element) -1)
        (`self.HandleforgetActor` _array_element)))))

(fn `CanSenseActor`
  (params (Actor :type "Actor Object Reference") (Sense :type "/Game/Blueprints/Characters/AI/Enums/E_AISense Enum" :default "NewEnumerator0"))
  (returns (Sensed :type Boolean) (Stimulis :type "AIStimulus Structure"))
  (bind _info (`AIPerceptionComponent.GetActorsPerception` (`self.AIPerception`) Actor))
  (for _array_element (`.LastSensedStimuli` (break `ActorPerceptionBlueprintInfo` _info))
    (bind _returnvalue (`AIPerceptionSystem.GetSenseClassForStimulus` _array_element))
    (if (== _returnvalue (select `/Game/Blueprints/Characters/AI/Enums/E_AISense` Sense :`NewEnumerator1` "/Script/AIModule.AISense_Sight" :`NewEnumerator2` "/Script/AIModule.AISense_Damage" :!type "Object Class Reference"))
      (return (`.bSuccessfullySensed` (break `AIStimulus` _array_element)) _array_element))))

(fn `GetCurrentState`
  (returns (State :type "/Game/Blueprints/Characters/AI/Enums/E_AIState Enum"))
  (return (cast `/Game/Blueprints/Characters/AI/Enums/E_AIState` (`BlackboardComponent.GetValueAsEnum` (`self.Blackboard`) (`self.StateKeyName`)))))

(fn `HandleforgetActor`
  (params (Actor :type "Actor Object Reference"))
  (`KismetArrayLibrary.Array_RemoveItem` (`self.KnownSeenActors`))
  (if (== Actor (`self.Attack Target`))
    (`self.SetStateAsPassive`)))

(fn `HandleSenseDamage`
  (params (Actor :type "Actor Object Reference"))
  (bind _sameteam (`self.OnSameTeam` Actor))
  (if (not _sameteam)
    (bind _state (`self.GetCurrentState`))
    (switch `/Game/Blueprints/Characters/AI/Enums/E_AIState` _state
      (:`NewEnumerator0`
        _)
      (:`NewEnumerator3`
        _))
    (`self.SetStateAsAttacking` Actor)))

(fn `HandleSensedSight`
  (params (Actor :type "Actor Object Reference"))
  (`KismetArrayLibrary.Array_AddUnique` (`self.KnownSeenActors`) Actor)
  (bind _state (`self.GetCurrentState`))
  (bind _sameteam (`self.OnSameTeam` Actor))
  (if (not _sameteam)
    (switch `/Game/Blueprints/Characters/AI/Enums/E_AIState` _state
      (:`NewEnumerator0`
        _)
      (:`NewEnumerator3`
        _))
    (`self.SetStateAsAttacking` Actor)))

(fn `OnSameTeam`
  (params (OtherActor :type "Actor Object Reference"))
  (returns (SameTeam :type Boolean))
  (bind _teamnumber (message `/Game/Blueprints/Characters/Blueprints/Interface/BPI_Damagable.GetTeamNumber` OtherActor))
  (bind _teamnumber_2 (message `/Game/Blueprints/Characters/Blueprints/Interface/BPI_Damagable.GetTeamNumber` (`self.K2_GetPawn`)))
  (return (== _teamnumber_2 _teamnumber)))

(fn `SetStateAsAttacking`
  (params (AttackTarget :type "Actor Object Reference"))
  (`BlackboardComponent.SetValueAsObject` (`self.Blackboard`) (`self.AttackTargetKyeName`) AttackTarget)
  (`BlackboardComponent.SetValueAsEnum` (`self.Blackboard`) (`self.StateKeyName`) (enumliteral `/Game/Blueprints/Characters/AI/Enums/E_AIState` "NewEnumerator1"))
  (set `self.Attack Target` AttackTarget))

(fn `SetStateAsDead`
  (`BlackboardComponent.SetValueAsEnum` (`self.Blackboard`) (`self.StateKeyName`) (enumliteral `/Game/Blueprints/Characters/AI/Enums/E_AIState` "NewEnumerator2")))

(fn `SetStateAsIdle`
  (`BlackboardComponent.SetValueAsEnum` (`self.Blackboard`) (`self.StateKeyName`) (enumliteral `/Game/Blueprints/Characters/AI/Enums/E_AIState` "NewEnumerator3")))

(fn `SetStateAsPassive`
  (`BlackboardComponent.SetValueAsEnum` (`self.Blackboard`) (`self.StateKeyName`) (enumliteral `/Game/Blueprints/Characters/AI/Enums/E_AIState` "NewEnumerator0")))

(fn `UserConstructionScript`)