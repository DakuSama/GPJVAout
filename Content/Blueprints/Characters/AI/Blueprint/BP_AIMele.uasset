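; BP_AIMele is a child AI character Blueprint that implements a melee auto attack.
; AutoAttack extends the parent event by playing an attack montage, then calls AttackEnd when it completes or is interrupted.
; Its Attack notify sphere-traces ahead for a pawn and compares team numbers through interface messages.
; A hit on another team sends blockable, parryable damage and reports a damage event to AI perception.
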(event `/Game/Blueprints/Characters/Blueprints/Interface/BPI_AIBase.AutoAttack`
  (params (AttackTarget :type "Actor Object Reference"))
  (bind _returnvalue (`self.K2_GetActorLocation`))
  (`parent.AutoAttack` AttackTarget)
  (bind _notifyname (`|PlayMontage` (`self.Mesh`) "/Game/Blueprints/Characters/AI/Animations/AM_AIBaseAttackA.AM_AIBaseAttackA")
    (:`OnCompleted`
      (`/Game/Blueprints/Characters/Blueprints/Interface/BPI_AIBase.AttackEnd` AttackTarget :!label _label))
    (:`OnInterrupted`
      (goto _label))
    (:`OnNotifyBegin`
      (switch `name` _notifyname
        (:`Attack`
          (bind _outhit (`KismetSystemLibrary.SphereTraceSingleForObjects` _returnvalue (+ _returnvalue (* (`self.GetActorForwardVector`) 150.0)) 50.0 (`|MakeArray` "ObjectTypeQuery3" :!type "EObjectTypeQuery Enum") false (`|MakeArray` self :!type "Actor Object Reference")))
          (bind (_bblockinghit _binitialoverlap _time _distance _location _impactpoint _normal _impactnormal _physmat _hitactor) (`GameplayStatics.BreakHitResult` _outhit))
          (bind _teamnumber (message `/Game/Blueprints/Characters/Blueprints/Interface/BPI_Damagable.GetTeamNumber` _hitactor))
          (bind _teamnumber_2 (message `/Game/Blueprints/Characters/Blueprints/Interface/BPI_Damagable.GetTeamNumber` self))
          (if (!= _teamnumber_2 _teamnumber)
            (message `/Game/Blueprints/Characters/Blueprints/Interface/BPI_Damagable.TakeDamage` _hitactor (make `/Game/Blueprints/Characters/Blueprints/Structures/S_DamageInfo` 40.0 "NewEnumerator1" "NewEnumerator0" false true true) self _hitactor)
            (`AISense_Damage.ReportDamageEvent` _hitactor self 50.0 (`self.K2_GetActorLocation`))))))))

(fn `UserConstructionScript`
  (`parent.UserConstructionScript`))